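; Player Blueprint that provides mouse look within a limited view range.
; On BeginPlay it clamps the player camera manager's yaw and pitch limits using the XRange and YRange variables.
; Mouse axis events add controller yaw and pitch input scaled by LookSpeed, with a PitchInversion multiplier on the vertical axis.
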(event EventBeginPlay
  (bind _returnvalue (Game|GetPlayerCameraManager 0))
  (bind _returnvalue_2 (Game|GetPlayerCameraManager 0))
  (Variables|/Script/Engine.PlayerCameraManager|SetViewYawMax _returnvalue_2 (.y (Variables|Default|GetxRange)))
  (Variables|/Script/Engine.PlayerCameraManager|SetViewYawMin _returnvalue_2 (.x (Variables|Default|GetxRange)))
  (Variables|/Script/Engine.PlayerCameraManager|SetViewPitchMax _returnvalue (.y (Variables|Default|GetyRange)))
  (Variables|/Script/Engine.PlayerCameraManager|SetViewPitchMin _returnvalue (.x (Variables|Default|GetyRange))))

(event Collision|EventActorBeginOverlap
  (params (OtherActor :type Actor%20Object%20Reference)))

(event EventTick
  (params (DeltaSeconds :type Float%20%28single-precision%29)))

(event Input|MouseEvents|MouseX
  (params (AxisValue :type Float%20%28single-precision%29))
  (Pawn|Input|AddControllerYawInput (* AxisValue (Variables|Default|GetlookSpeed))))

(event Input|MouseEvents|MouseY
  (params (AxisValue :type Float%20%28single-precision%29))
  (Pawn|Input|AddControllerPitchInput (* AxisValue (Variables|Default|GetlookSpeed) (Variables|Default|GetpitchInversion))))

(fn ConstructionScript)