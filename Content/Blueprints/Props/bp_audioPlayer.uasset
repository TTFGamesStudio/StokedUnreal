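; Fire-and-forget audio player actor that plays a given sound clip and removes itself when playback finishes.
; A startAudio event assigns the clip to its Audio component, sets a started flag and plays it from the beginning.
; Tick polls the component once started and destroys the actor when the sound stops playing.
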(event Custom|startAudio
  (params (clip :type Sound%20Wave%20Object%20Reference))
  (bind _audio (Variables|Default|GetAudio))
  (Audio|Components|Audio|SetSound _audio clip)
  (Variables|Default|SetaudioStarted true)
  (Audio|Components|Audio|Play _audio 0.0))

(event EventBeginPlay)

(event Collision|EventActorBeginOverlap
  (params (OtherActor :type Actor%20Object%20Reference)))

(event EventTick
  (params (DeltaSeconds :type Float%20%28single-precision%29))
  (if (Variables|Default|GetaudioStarted)
    (if (not (Audio|Components|Audio|IsPlaying (Variables|Default|GetAudio)))
      (Actor|DestroyActor))))

(fn ConstructionScript)