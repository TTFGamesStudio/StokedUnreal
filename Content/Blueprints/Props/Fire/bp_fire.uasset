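; Fire prop Blueprint that shows fire through a Niagara effect, a point light and a sound.
; Every Tick, a single FireStrength value scales the Niagara fireStrength parameter, the light intensity and the sound volume together.
; The Blueprint only reads FireStrength and contains no logic that changes it.
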(event EventBeginPlay)

(event Collision|EventActorBeginOverlap
  (params (OtherActor :type Actor%20Object%20Reference)))

(event EventTick
  (params (DeltaSeconds :type Float%20%28single-precision%29))
  (Niagara|SetNiagaraVariable(Float) (Variables|Default|GetNiagara) "fireStrength" (* 1e+02 (Variables|Default|GetfireStrength)))
  (Rendering|Components|Light|SetIntensity (Variables|Default|GetPointLight) (* 5e+03 (Variables|Default|GetfireStrength)))
  (Audio|Components|Audio|SetVolumeMultiplier (Variables|Default|GetfireSound) (Variables|Default|GetfireStrength) :!class /Script/Engine.AudioComponent))

(fn ConstructionScript)