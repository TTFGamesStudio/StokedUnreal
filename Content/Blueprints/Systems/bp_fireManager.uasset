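; Fire manager actor that tracks the strength of a fire and a limited supply of logs for stoking it.
; Each tick it decays strength in proportion to its current value, clamps it to 0–1 and passes it to the Fire actor.
; Releasing Stoke Fire spends a log only if strength has room for the full gain, then plays a drop sound and spawns a FireStoke actor.
; Six log props show or hide to match the remaining count.
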(event EventBeginPlay)

(event Collision|EventActorBeginOverlap
  (params (OtherActor :type Actor%20Object%20Reference)))

(event EventTick
  (params (DeltaSeconds :type Float%20%28single-precision%29))
  (Variables|Default|SetDelta%20Seconds DeltaSeconds)
  (bind _output_get (Variables|FireStats|SetfireStrength (- (Variables|FireStats|GetfireStrength) (* DeltaSeconds (Variables|Default|GetfireDrain) (Variables|FireStats|GetfireStrength)))))
  (bind _output_get_2 (Variables|FireStats|SetfireStrength (Math|Float|Clamp(Float) _output_get)))
  (Variables|/Game/Blueprints/Props/Fire/bp_fire.bp_fire_C|SetfireStrength (Variables|Default|Getfire) _output_get_2))

(event Input|ActionEvents|InputActionStokeFire
  (params (Key :type Key%20Structure :default "None"))
  (:Released
    (CallFunction|AddLog)))

(fn ConstructionScript)

(fn UpdateLogs
  (CallFunction|UpdateLog (Variables|FirewoodReferences|Getlog1) 1)
  (CallFunction|UpdateLog (Variables|FirewoodReferences|Getlog2) 2)
  (CallFunction|UpdateLog (Variables|FirewoodReferences|Getlog3) 3)
  (CallFunction|UpdateLog (Variables|FirewoodReferences|Getlog4) 4)
  (CallFunction|UpdateLog (Variables|FirewoodReferences|Getlog5) 5)
  (CallFunction|UpdateLog (Variables|FirewoodReferences|Getlog6) 6))

(fn UpdateLog
  (params (log :type Bp%20Firewood%20Object%20Reference) (logNumber :type Integer))
  (if (< (Variables|FireStats|Getlogs) logNumber)
    (Rendering|SetVisibility (Variables|/Game/Blueprints/Props/Logs/bp_firewood.bp_firewood_C|Getlog1 log) false false)
    (else
      (Rendering|SetVisibility (Variables|/Game/Blueprints/Props/Logs/bp_firewood.bp_firewood_C|Getlog1 log) true false))))

(fn AddLog
  (bind _fire (Variables|Default|Getfire))
  (bind _returnvalue (Transformation|GetActorTransform _fire))
  (if (> (Variables|FireStats|Getlogs) 0)
    (if (> (- (Class|KismetSystemLibrary|MakeLiteralInteger 1) (Variables|FireStats|GetfireStrength)) (Variables|FireStats|GetfireGainWithLog))
      (Variables|FireStats|Setlogs (- (Variables|FireStats|Getlogs) 1))
      (Variables|FireStats|SetfireStrength (+ (Variables|FireStats|GetfireStrength) (Variables|FireStats|GetfireGainWithLog)))
      (CallFunction|UpdateLogs)
      (bind _returnvalue_2 (Game|SpawnActorfromClass "/Game/Blueprints/Props/bp_audioPlayer.bp_audioPlayer_C" _returnvalue "Undefined" "MultiplyWithRoot" 0 0))
      (Default|StartAudio _returnvalue_2 "/Game/Audio/ES_Impact_Log_Drop_1_-_SFX_Producer.ES_Impact_Log_Drop_1_-_SFX_Producer")
      (Game|SpawnActorfromClass "/Game/Blueprints/Props/fireStoke.fireStoke_C" _returnvalue "Undefined" "MultiplyWithRoot" 0 0))))